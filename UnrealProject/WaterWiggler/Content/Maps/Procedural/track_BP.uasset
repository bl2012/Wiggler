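; Procedural track segment with a boat spline path and an attach transform for chaining, used by the endless and defined-track wiggler game modes.
; Boat collision advances the ChrisCraft to its next track once, if this segment is its current one.
; A later worm overlap re-arms that trigger, also spawning a track and destroying this segment in endless mode.
; The event graph holds only empty events and disconnected timeline and debug logic.
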(event Custom|ChooseTimeline)

(event EventTick
  (params (DeltaSeconds :type Float%20%28single-precision%29)))

(fn ConstructionScript
  (Variables|Default|Setdist_along_spline 0.0)
  (Variables|Default|SettriggerNext true))

(fn GetAttachTransform
  (return (Transformation|GetWorldTransform (Variables|Default|Getattach_point))))

(fn CheckActiveTrack
  (params (boat :type Chris%20Craft%20Blueprint%20Object%20Reference))
  (return (== (Variables|/Game/VehicleBP/ChrisCraft/ChrisCraft_Blueprint.ChrisCraft_Blueprint_C|GetcurrentTrack boat) self)))

(fn BoatCollisionStuff
  (params (OtherActor :type Actor%20Object%20Reference))
  (bind _aschris_craft_blueprint (Utilities|Casting|CastToChrisCraft_Blueprint OtherActor))
  (bind _iscurrenttrack (CallFunction|CheckActiveTrack _aschris_craft_blueprint))
  (Utilities|FlowControl|Sequence
    (:then_0
      (if (and _iscurrenttrack (Variables|Default|GettriggerNext))
        (Default|NextTrack _aschris_craft_blueprint)
        (Variables|Default|SettriggerNext false)
        (Development|PrintString "next track")))
    (:then_1
      (Development|PrintString "boat collision"))))

(fn WormCollisionStuff
  (params (OtherActor :type Actor%20Object%20Reference))
  (bind _returnvalue (Game|GetGameMode))
  (if (not (Variables|Default|GettriggerNext))
    (Development|PrintString "overlap worm")
    (Utilities|FlowControl|Sequence
      (:then_0
        (bind _asgm_wiggler_endless (Utilities|Casting|CastToGM_wiggler_endless _returnvalue))
        (Default|SpawnTrack _asgm_wiggler_endless)
        (Actor|DestroyActor))
      (:then_1
        (Utilities|Casting|CastToGM_wiggler_definedTrack _returnvalue)))
    (Variables|Default|SettriggerNext true)
    (Development|PrintString "TriggerNext true")))

(fn CheckLastTrack
  (params (GameMode :type Game%20Mode%20Wiggler%20Object%20Reference))
  (bind _tracklist (Variables|/Game/Blueprints/GameModes/GameMode_wiggler.GameMode_wiggler_C|GettrackList GameMode))
  (return (== (Utilities|Array|Get(acopy) _tracklist (- (Utilities|Array|Length _tracklist) 1)) self)))