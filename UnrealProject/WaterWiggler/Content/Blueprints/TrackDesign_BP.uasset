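; TrackDesign_BP holds a designed Track list and contains logic to build it as a chain of track pieces, though that logic is disconnected and never runs.
; The unwired graph starts at the actor tagged ChrisCraft and has GameMode_definedTrack add each piece at the previous one's AttachPoint.
; It then sets the ChrisCraft's CurrentTrack to the first piece.
; The construction script itself does nothing.
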(fn ConstructionScript)