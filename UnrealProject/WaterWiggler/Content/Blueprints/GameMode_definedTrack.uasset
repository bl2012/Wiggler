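; Game mode that builds a predefined track from modular pieces at level start.
; BeginPlay walks the TrackDesign list, calls AddTrack to spawn each piece at the next spawn transform, and records it in TrackList.
; Each piece's AttachPoint is read to position and orient the following one.
; Disconnected nodes hold unused logic for piece visibility and setting the ChrisCraft's current track; AddTrack's return node is also unwired.
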(event EventBeginPlay
  (bind _trackdesign (Variables|Default|GettrackDesign))
  ;[0.3208 0.8392 0.8019 1 50] Level Setup
  (for _index (range 0 (- (Utilities|Array|Length _trackdesign) 1))
    (bind _spawned_track (CallFunction|AddTrack (Utilities|Array|Get(acopy) _trackdesign _index)))
    (Utilities|Array|Add (Variables|Default|GettrackList) _spawned_track)
    (Variables|Default|SetnextSpawnPoint (Transformation|GetWorldLocation (Variables|/Game/Maps/Procedural/track_BP.track_BP_C|Getattach_point _spawned_track)))
    (Variables|Default|SetnextSpawnRotation (Transformation|GetWorldRotation (Variables|/Game/Maps/Procedural/track_BP.track_BP_C|Getattach_point _spawned_track)))))

(fn ConstructionScript)

(fn AddTrack
  (params (TrackType :type Track%20BP%20Class%20Reference))
  ;[1 1 1] spawn actor of the input track type at the next spawn point
  (bind _returnvalue (Game|SpawnActorfromClass TrackType (Math|Transform|MakeTransform (Variables|Default|GetnextSpawnPoint) (Variables|Default|GetnextSpawnRotation)) "Undefined" 0 0)))