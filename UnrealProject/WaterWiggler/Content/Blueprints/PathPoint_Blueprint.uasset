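; Waypoint actor on the path followed by the ChrisCraft boat.
; It caches the GameManager, found by actor tag, on BeginPlay.
; When a ChrisCraft overlaps it and it is that boat's current destination, it flags the boat as turning and calls the manager's LoopPoints and NextPathPoint.
; When the boat leaves, it clears the turning flag and marks itself visited.
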(event EventBeginPlay
  (bind _outactors (Actor|GetAllActorswithTag "GameManager"))
  (bind _asgame_manager (Utilities|Casting|CastToGameManager (Utilities|Array|Get(acopy) _outactors)))
  (Variables|Default|SetManager _asgame_manager))

(event Collision|EventActorBeginOverlap
  (params (OtherActor :type Actor%20Object%20Reference))
  (bind _manager (Variables|Default|GetManager))
  (bind _aschris_craft_blueprint (Utilities|Casting|CastToChrisCraft_Blueprint OtherActor))
  (if (== self (Variables|/Game/VehicleBP/ChrisCraft/ChrisCraft_Blueprint.ChrisCraft_Blueprint_C|GetDest _aschris_craft_blueprint))
    (Variables|/Game/VehicleBP/ChrisCraft/ChrisCraft_Blueprint.ChrisCraft_Blueprint_C|SetbIsTurning _aschris_craft_blueprint true)
    (Default|LoopPoints _manager self)
    (Default|NextPathPoint _manager)))

(event Collision|EventActorEndOverlap
  (params (OtherActor :type Actor%20Object%20Reference))
  (bind _aschris_craft_blueprint (Utilities|Casting|CastToChrisCraft_Blueprint OtherActor))
  (Variables|/Game/VehicleBP/ChrisCraft/ChrisCraft_Blueprint.ChrisCraft_Blueprint_C|SetbIsTurning _aschris_craft_blueprint false)
  (Variables|Default|SetVisited true))

(fn ConstructionScript
  (Variables|Default|SetVisited false))