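; Deprecated game mode that builds a predefined track in front of the player craft at BeginPlay.
; It reads the ordered list of piece classes from the level's TrackDesign_BP and starts at the transform of the ChrisCraft-tagged actor.
; AddTrack spawns each piece, whose AttachPoint then sets the location and rotation for the next.
; The first spawned piece becomes the craft's CurrentTrack.
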(event EventBeginPlay
  (bind _tracklist (Variables|Default|GettrackList))
  (bind _output (Utilities|Array|Get(acopy) _tracklist))
  (bind _outactors (Actor|GetAllActorsOfClass "/Game/Blueprints/TrackDesign_BP.TrackDesign_BP_C"))
  (Variables|Default|SettrackDesign (Variables|/Game/Blueprints/TrackDesign_BP.TrackDesign_BP_C|Gettrack (Utilities|Array|Get(acopy) _outactors)))
  (bind _outactors_2 (Actor|GetAllActorswithTag "ChrisCraft"))
  (bind _aschris_craft_blueprint (Utilities|Casting|CastToChrisCraft_Blueprint (Utilities|Array|Get(acopy) _outactors_2)))
  (Variables|Default|SetnextSpawnPoint (Transformation|GetWorldLocation (Variables|/Script/Engine.Actor|GetRootComponent _aschris_craft_blueprint)))
  (Variables|Default|SetnextSpawnRotation (Transformation|GetWorldRotation (Variables|/Script/Engine.Actor|GetRootComponent _aschris_craft_blueprint)))
  (for _index (range 0 (- (Utilities|Array|Length (Variables|Default|GettrackDesign)) 1))
    (bind _spawned_track (CallFunction|AddTrack (Utilities|Array|Get(acopy) (Variables|Default|GettrackDesign) _index)))
    (Utilities|Array|Add (Variables|Default|GettrackList) _spawned_track)
    (Variables|Default|SetnextSpawnPoint (Transformation|GetWorldLocation (Variables|/Game/Maps/Procedural/track_BP.track_BP_C|Getattach_point _spawned_track)))
    (Variables|Default|SetnextSpawnRotation (Transformation|GetWorldRotation (Variables|/Game/Maps/Procedural/track_BP.track_BP_C|Getattach_point _spawned_track))))
  (bind _output_get (Variables|/Game/VehicleBP/ChrisCraft/ChrisCraft_Blueprint.ChrisCraft_Blueprint_C|SetcurrentTrack _aschris_craft_blueprint _output))
  (|SetBy-RefVar _output_get _output))

(fn ConstructionScript)

(fn AddTrack
  (params (TrackType :type Track%20BP%20Class%20Reference))
  ;[1 1 1] spawn actor of the input track type at the next spawn point
  (bind _returnvalue (Game|SpawnActorfromClass TrackType (Math|Transform|MakeTransform (Variables|Default|GetnextSpawnPoint) (Variables|Default|GetnextSpawnRotation)) "Undefined" 0 0))
  (return _returnvalue))