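; Deprecated endless-mode GameMode that builds a track from chained, randomly chosen pieces at BeginPlay.
; It spawns a forward starter, then a fixed count of random TrackTypes, each placed at the previous piece's AttachPoint and stored in TrackList.
; Pieces spawn hidden, the first three are revealed, and the tagged ChrisCraft receives the starter as CurrentTrack.
; The debug print re-rolls the random index, so its logged type can differ from the spawned piece.
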(event Custom|SpawnTrack
  (bind _track_types (Variables|Default|Gettrack_types))
  (bind _returnvalue (Utilities|Array|Length _track_types))
  (bind _returnvalue_2 (- _returnvalue 1))
  (bind _returnvalue_3 (Math|Random|RandomIntegerinRange 0 _returnvalue_2))
  (bind _output (Utilities|Array|Get(acopy) _track_types _returnvalue_3))
  ;[0.5029 0.3467 0.8388 1 50] Spawn Track
  ;;[1 1 1] spawn random track type
  (bind _spawned_track (CallFunction|AddTrack _output))
  ;;[1 1 1] set spawn loc/rot to the end of the spawned track
  (Variables|Default|SetnextSpawnPoint (Transformation|GetWorldLocation (Variables|/Game/Maps/Procedural/track_BP.track_BP_C|Getattach_point _spawned_track)))
  (Variables|Default|SetnextSpawnRotation (Transformation|GetWorldRotation (Variables|/Game/Maps/Procedural/track_BP.track_BP_C|Getattach_point _spawned_track)))
  ;;[1 1 1] add spawned track to track list
  (Utilities|Array|Add (Variables|Default|Gettrack_list) _spawned_track)
  (Development|PrintString (Utilities|String|Append "track spawned: " (Utilities|GetClassDisplayName _output))))

(event EventBeginPlay
  (bind _track_list (Variables|Default|Gettrack_list))
  ;[0.3208 0.8392 0.8019 1 50] Level Setup
  (Utilities|FlowControl|Sequence
    (:then_0
      (Variables|Default|SetnumTrackPieces 5))
    (:then_1
      ;;[1 1 1] spawn beginning track, set attach point as next spawn point, add track to track list
      (bind _spawned_track (CallFunction|AddTrack "/Game/Maps/Procedural/track_forward.track_forward_C"))
      (Variables|Default|SetnextSpawnPoint (Transformation|GetWorldLocation (Variables|/Game/Maps/Procedural/track_BP.track_BP_C|Getattach_point _spawned_track)))
      (Variables|Default|SetnextSpawnRotation (Transformation|GetWorldRotation (Variables|/Game/Maps/Procedural/track_BP.track_BP_C|Getattach_point _spawned_track)))
      (Utilities|Array|Add _track_list _spawned_track)
      ;;[1 1 1] spawn the predetermined number of track pieces
      (for _index (range 0 (- (Variables|Default|GetnumTrackPieces) 1))
        (CallFunction|SpawnTrack))
      (for _index_2 (range 0 2)
        (Rendering|SetVisibility (Variables|/Game/Maps/Procedural/track_BP.track_BP_C|GetDefaultSceneRoot (Utilities|Array|Get(acopy) _track_list _index_2)) true true)
        (|SetBy-RefVar (Utilities|Array|Get(acopy) _track_list _index_2) (Utilities|Array|Get(acopy) _track_list _index_2))))
    (:then_2
      ;;[1 1 1] set first track as current track in the active ChrisCraft
      (bind _outactors (Actor|GetAllActorswithTag "ChrisCraft"))
      (bind _aschris_craft_blueprint (Utilities|Casting|CastToChrisCraft_Blueprint (Utilities|Array|Get(acopy) _outactors)))
      (Variables|/Game/VehicleBP/ChrisCraft/ChrisCraft_Blueprint.ChrisCraft_Blueprint_C|SetcurrentTrack _aschris_craft_blueprint _spawned_track))))

(fn ConstructionScript)

(fn AddTrack
  (params (TrackType :type Track%20BP%20Class%20Reference))
  ;[1 1 1] spawn actor of the input track type at the next spawn point
  (bind _returnvalue (Game|SpawnActorfromClass TrackType (Math|Transform|MakeTransform (Variables|Default|GetnextSpawnPoint) (Variables|Default|GetnextSpawnRotation)) "Undefined" 0 0))
  (Rendering|SetVisibility (Variables|/Game/Maps/Procedural/track_BP.track_BP_C|GetDefaultSceneRoot _returnvalue) false true)
  (return _returnvalue))