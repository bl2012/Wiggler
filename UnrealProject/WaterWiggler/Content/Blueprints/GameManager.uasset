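; GameManager blueprint that holds an ordered Path of points and feeds destinations to the ChrisCraft actor.
; On BeginPlay, NextPathPoint finds the first actor tagged ChrisCraft and sets its Dest and NextDest from the first two Path entries.
; LoopPoints moves a visited point to the end of Path and clears its Visited flag, cycling the route.
; The construction script adds the GameManager tag for lookup.
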(event EventBeginPlay
  (CallFunction|NextPathPoint))

(fn ConstructionScript
  (bind _returnvalue (Utilities|String|StringToName "GameManager"))
  (bind _tags (Variables|Actor|GetTags))
  (if (not (Utilities|Array|ContainsItem _tags _returnvalue))
    (Utilities|Array|Add _tags _returnvalue)))

(fn NextPathPoint
  (bind _path (Variables|Default|GetPath))
  (bind _outactors (Actor|GetAllActorswithTag "ChrisCraft"))
  (bind _aschris_craft_blueprint (Utilities|Casting|CastToChrisCraft_Blueprint (Utilities|Array|Get(acopy) _outactors)))
  (Variables|/Game/VehicleBP/ChrisCraft/ChrisCraft_Blueprint.ChrisCraft_Blueprint_C|SetDest _aschris_craft_blueprint (Utilities|Array|Get(acopy) _path))
  (Variables|/Game/VehicleBP/ChrisCraft/ChrisCraft_Blueprint.ChrisCraft_Blueprint_C|SetNext_Dest _aschris_craft_blueprint (Utilities|Array|Get(acopy) _path 1)))

(fn LoopPoints
  (params (VisitedPoint :type Path%20Point%20Blueprint%20Object%20Reference))
  (bind _path (Variables|Default|GetPath))
  (bind _returnvalue (Utilities|Array|RemoveItem _path VisitedPoint))
  (if _returnvalue
    (Utilities|Array|Add _path VisitedPoint)
    (Variables|/Game/Blueprints/PathPoint_Blueprint.PathPoint_Blueprint_C|SetVisited VisitedPoint false)))