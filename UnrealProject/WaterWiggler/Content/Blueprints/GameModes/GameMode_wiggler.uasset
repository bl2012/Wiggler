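; Game mode for the wiggler game, providing shared track spawning for its endless and defined-track modes.
; AddTrack spawns an actor of the given track type at the stored next spawn location and rotation, without updating either.
; Casts on the active game mode decide visibility: endless mode hides the new track's root and children before returning it, while defined-track mode returns it untouched.
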(event EventBeginPlay)

(event EventTick
  (params (DeltaSeconds :type Float%20%28single-precision%29)))

(fn ConstructionScript)

(fn AddTrack
  (params (track_type :type Track%20BP%20Class%20Reference))
  (bind _returnvalue (Game|GetGameMode))
  ;[1 1 1] spawn actor of the input track type at the next spawn point
  (bind _returnvalue_2 (Game|SpawnActorfromClass track_type (Math|Transform|MakeTransform (Variables|Default|GetnextSpawnPoint) (Variables|Default|GetnextSpawnRotation)) "Undefined" 0 0))
  (Utilities|FlowControl|Sequence
    (:then_0
      (Utilities|Casting|CastToGM_wiggler_endless _returnvalue)
      (Rendering|SetVisibility (Variables|/Game/Maps/Procedural/track_BP.track_BP_C|GetDefaultSceneRoot _returnvalue_2) false true))
    (:then_1
      (Utilities|Casting|CastToGM_wiggler_definedTrack _returnvalue)))
  (return _returnvalue_2))