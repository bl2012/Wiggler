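; Base enemy character Blueprint, with only placeholder movement and detection logic so far.
; On BeginPlay it uses SimpleMoveToLocation to head for a fixed diagonal offset from its starting position.
; PawnSensing prints a debug message when it sees a ChrisCraft_Blueprint pawn.
; AIMoveTo, DestroyActor and a random point in the craft's current-track spawn area are left unconnected, so the BeginPlay actor lookup has no effect.
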(event OnSeePawn(PawnSensing)
  (params (Pawn :type Pawn%20Object%20Reference))
  (Utilities|Casting|CastToChrisCraft_Blueprint Pawn)
  (Development|PrintString "I see you"))

(event EventBeginPlay
  (bind _returnvalue (Transformation|GetActorLocation))
  (bind (_x _y _z) (Math|Vector|BreakVector _returnvalue))
  (bind _outactors (Actor|GetAllActorsOfClass "/Game/VehicleBP/ChrisCraft/ChrisCraft_Blueprint.ChrisCraft_Blueprint_C"))
  (AI|Navigation|SimpleMovetoLocation (Pawn|GetController self) (Math|Vector|MakeVector (+ _x 1e+03) (+ _y 1e+03) _z)))

(event Collision|EventActorBeginOverlap
  (params (OtherActor :type Actor%20Object%20Reference)))

(event EventTick
  (params (DeltaSeconds :type Float%20%28single-precision%29)))

(fn ConstructionScript)