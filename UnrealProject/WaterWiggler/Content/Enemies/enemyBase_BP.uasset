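; Base enemy actor, shown as a piranha that loops its swim animation from BeginPlay.
; On overlap, a sequence casts the other actor to the worm and boat Blueprints and prints a matching "ouch" message, then prints the actor's name.
; The Hit event jumps into that same name print, which reads the overlap event's actor.
; Contact responses are debug prints only, with no damage or movement logic.
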(event EventBeginPlay
  (Components|Animation|PlayAnimation (Variables|Default|Getenemy_mesh) "/Game/Enemies/piranha_swim_Anim.piranha_swim_Anim" true))

(event Collision|EventActorBeginOverlap
  (params (OtherActor :type Actor%20Object%20Reference))
  (Utilities|FlowControl|Sequence
    (:then_0
      (Utilities|Casting|CastToWorm_Blueprint OtherActor)
      (Development|PrintString "worm ouch"))
    (:then_1
      (Utilities|Casting|CastToChrisCraft_Blueprint OtherActor)
      (Development|PrintString "boat ouch"))
    (:then_2
      (Development|PrintString (Utilities|GetDisplayName OtherActor)))))

(event Collision|EventHit
  (params (MyComp :type Primitive%20Component%20Object%20Reference) (Other :type Actor%20Object%20Reference) (OtherComp :type Primitive%20Component%20Object%20Reference) (bSelfMoved :type Boolean) (HitLocation :type Vector :default "0, 0, 0") (HitNormal :type Vector :default "0, 0, 0") (NormalImpulse :type Vector :default "0, 0, 0") (Hit :type Hit%20Result%20Structure%20%28by%20ref%29))
  (Development|PrintString (Utilities|GetDisplayName (stale Collision|EventActorBeginOverlap OtherActor))))

(fn ConstructionScript)