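; Track design actor that turns an array of forward, left and right pieces into a spline path.
; Its construction script registers it as CurrentTrack on the ChrisCraft_Blueprint actor found in the level.
; DrawTrack creates a spline component at runtime and walks the Track array, adding points at fixed offsets for each direction.
; DrawTrack prints rotation and completion debug messages and is not called within this Blueprint.
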(event EventBeginPlay)

(fn ConstructionScript
  (bind _returnvalue (Actor|GetActorOfClass "/Game/VehicleBP/ChrisCraft/ChrisCraft_Blueprint.ChrisCraft_Blueprint_C"))
  (Variables|/Game/VehicleBP/ChrisCraft/ChrisCraft_Blueprint.ChrisCraft_Blueprint_C|SetcurrentTrack _returnvalue self))

(fn DrawTrack
  (bind _returnvalue (AddComponent|AddSplineComponent false))
  (bind _output_get (Variables|Default|SetnewPointLoc "200.000000, 0, 0"))
  (Spline|AddSplinePoint _returnvalue _output_get "Local" true)
  (for (_array_element _array_index) (Variables|Default|Gettrack)
    (Variables|Default|SetoldPointLoc (Variables|Default|GetnewPointLoc))
    (bind _output_get_2 (Variables|Default|SetnewPointLoc (+ (* (Math|Vector|GetForwardVector _returnvalue) 100) (Variables|Default|GetoldPointLoc))))
    (Spline|AddSplinePoint _returnvalue _output_get_2 "Local" true)
    (if (== _array_element "/Game/Maps/Procedural/track_forward.track_forward_C")
      (Variables|Default|SetnewPointLoc (+ (Math|Vector|MakeVector 1e+02 0.0 0.0) (Variables|Default|GetnewPointLoc)))
      (Class|SplineComponent|AddPoint _returnvalue (Utilities|Struct|MakeSplinePoint (Math|Conversions|ToFloat(Integer) _array_index) (stale _output_get_3) "0.000000,0.000000,0.000000" "0.000000,0.000000,0.000000" (Math|Rotator|MakeRotfromXY (Variables|Default|GetoldPointLoc) (stale _output_get_3))) true :!label _label)
      (Development|PrintString (Utilities|String|Append "rotation: " (Utilities|String|ToString(Rotator) (Math|Rotator|MakeRotfromXY (Variables|Default|GetoldPointLoc) (stale _output_get_3)))) true true "(R=0.000000,G=0.660000,B=1.000000,A=1.000000)" 1e+01)
      (elif (== _array_element "/Game/Maps/Procedural/track_left.track_left_C")
        (Variables|Default|SetnewPointLoc (+ (Math|Vector|MakeVector 0.0 -1e+02 0.0) (Variables|Default|GetnewPointLoc)))
        (goto _label)
        (elif (== _array_element "/Game/Maps/Procedural/track_right.track_right_C")
          (bind _output_get_3 (Variables|Default|SetnewPointLoc (+ (Math|Vector|MakeVector 0.0 1e+02 0.0) (Variables|Default|GetnewPointLoc))))
          (goto _label)))))
  (Development|PrintString "track_complete"))