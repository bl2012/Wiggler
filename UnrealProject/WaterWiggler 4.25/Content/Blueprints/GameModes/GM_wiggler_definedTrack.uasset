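; Game mode that builds a boat track at BeginPlay from a predefined layout, then runs its parent's BeginPlay.
; It reads the piece list from the second TrackDesign_BP found in the level and starts at the transform of the actor tagged ChrisCraft.
; Each piece spawned through AddTrack joins TrackList, and its AttachPoint sets the next spawn transform.
; The first piece becomes the boat's CurrentTrack.
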(event EventBeginPlay
  (bind _tracklist (Variables|Default|GettrackList))
  (bind _output (Utilities|Array|Get(acopy) _tracklist))
  (Utilities|FlowControl|Sequence
    (:then_0
      ;[1 0.9567 0.4656 1 50] set up track as defined in the TrackDesignBP that exists in the level
      ;;[1 1 1] set references to the track design and boat
      (bind _outactors (Actor|GetAllActorsOfClass "/Game/Blueprints/TrackDesign_BP.TrackDesign_BP_C"))
      (Variables|Default|SettrackDesign (Variables|/Game/Blueprints/TrackDesign_BP.TrackDesign_BP_C|Gettrack (Utilities|Array|Get(acopy) _outactors 1)))
      (bind _outactors_2 (Actor|GetAllActorswithTag "ChrisCraft"))
      (bind _aschris_craft_blueprint (Utilities|Casting|CastToChrisCraft_Blueprint (Utilities|Array|Get(acopy) _outactors_2)))
      ;;[1 1 1] set initial points for spawning track
      (Variables|Default|SetnextSpawnPoint (Transformation|GetWorldLocation (Variables|/Script/Engine.Actor|GetRootComponent _aschris_craft_blueprint)))
      (Variables|Default|SetnextSpawnRotation (Transformation|GetWorldRotation (Variables|/Script/Engine.Actor|GetRootComponent _aschris_craft_blueprint)))
      ;;[1 1 1] loop through all elements of the track design
      (for _index (range 0 (- (Utilities|Array|Length (Variables|Default|GettrackDesign)) 1))
        ;;[1 1 1] spawn given track and add it to the track list
        (bind _spawned_track (CallFunction|AddTrack (Utilities|Array|Get(acopy) (Variables|Default|GettrackDesign) _index)))
        ;;[1 1 1] use attach point of the track to update the spawn point for the next element of the track
        (Utilities|Array|Add (Variables|Default|GettrackList) _spawned_track)
        (Variables|Default|SetnextSpawnPoint (Transformation|GetWorldLocation (Variables|/Game/Maps/Procedural/track_BP.track_BP_C|Getattach_point _spawned_track)))
        (Variables|Default|SetnextSpawnRotation (Transformation|GetWorldRotation (Variables|/Game/Maps/Procedural/track_BP.track_BP_C|Getattach_point _spawned_track))))
      ;;[1 1 1] after track is spawned, set the first element of the track as the boat's current track
      (bind _output_get (Variables|/Game/VehicleBP/ChrisCraft/ChrisCraft_Blueprint.ChrisCraft_Blueprint_C|SetcurrentTrack _aschris_craft_blueprint _output))
      (|SetBy-RefVar _output_get _output))
    (:then_1
      (|CallParentFunction))))

(fn ConstructionScript
  (|CallParentFunction))