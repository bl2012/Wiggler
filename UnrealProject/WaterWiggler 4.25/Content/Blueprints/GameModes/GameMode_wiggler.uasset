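; GameMode_wiggler is a game mode that spawns track pieces and enemies, with behavior for endless and defined-track variants.
; AddTrack spawns a track at the next spawn point and hides it in endless mode.
; SpawnEnemy places random enemy types inside a track's spawn area, reusing pooled actors once over five instances exist, though the type is re-rolled at each use.
; SendToPool hides enemies for reuse; only piranhas have a pool.
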(event EventBeginPlay)

(event EventTick
  (params (DeltaSeconds :type Float%20%28single-precision%29)))

(fn ConstructionScript)

(fn AddTrack
  (params (track_type :type Track%20BP%20Class%20Reference))
  (bind _returnvalue (Game|GetGameMode))
  ;[1 1 1] spawn actor of the input track type at the next spawn point
  (bind _returnvalue_2 (Game|SpawnActorfromClass track_type (Math|Transform|MakeTransform (Variables|Default|GetnextSpawnPoint) (Variables|Default|GetnextSpawnRotation)) "Undefined" 0 0))
  (Utilities|FlowControl|Sequence
    (:then_0
      (Utilities|Casting|CastToGM_wiggler_endless _returnvalue)
      (Rendering|SetVisibility (Variables|/Game/Maps/Procedural/track_BP.track_BP_C|GetDefaultSceneRoot _returnvalue_2) false true))
    (:then_1
      (Utilities|Casting|CastToGM_wiggler_definedTrack _returnvalue)))
  (return _returnvalue_2))

(fn SpawnEnemy
  (params (track :type Track%20BP%20Object%20Reference%20%28by%20ref%29))
  (bind _enemytypes (Variables|Default|GetenemyTypes))
  (bind _enemy_spawn_area (Variables|/Game/Maps/Procedural/track_BP.track_BP_C|Getenemy_spawn_area track))
  (bind _returnvalue (Utilities|Array|Length _enemytypes))
  (bind _returnvalue_2 (Components|Box|GetScaledBoxExtent _enemy_spawn_area))
  (bind _returnvalue_3 (Transformation|GetWorldLocation _enemy_spawn_area))
  (bind _returnvalue_4 (Math|Random|RandomPointinBoundingBox _returnvalue_3 _returnvalue_2))
  (bind _returnvalue_5 (- _returnvalue 1))
  (bind _returnvalue_6 (Math|Random|RandomIntegerinRange 0 _returnvalue_5))
  (bind _returnvalue_7 (Math|Conversions|ToTransform(Vector) _returnvalue_4))
  (bind _output (Utilities|Array|Get(acopy) _enemytypes _returnvalue_6))
  (bind _outactors (Actor|GetAllActorsOfClass _output))
  (Development|PrintString (Utilities|String|Append (Utilities|String|ToString(Integer) (Utilities|Array|Length _outactors)) " total " (Utilities|GetClassDisplayName _output)))
  (if (> (Utilities|Array|Length _outactors) 5)
    ;[1 1 1] "spawn" from pool rather than creating new actor
    (bind _enemypool (CallFunction|SelectPool _output))
    (Transformation|SetActorTransform (Utilities|Array|Get(acopy) _enemypool (- (Utilities|Array|Length _enemypool) 1)) _returnvalue_7)
    (Rendering|SetActorHiddenInGame (Utilities|Array|Get(acopy) _enemypool (- (Utilities|Array|Length _enemypool) 1)) false)
    (Utilities|Array|RemoveIndex _enemypool (- (Utilities|Array|Length _enemypool) 1))
    (Development|PrintString "removed from pool")
    (else
      ;[1 1 1] if 5 or less instances of an enemy exist, spawn a new one
      (Game|SpawnActorfromClass _output _returnvalue_7 "AdjustIfPossibleButAlwaysSpawn" 0 0)
      (Development|PrintString "enemy spawned" true true "(R=0.000000,G=0.660000,B=1.000000,A=1.000000)" 1e+01))))

(fn SelectPool
  (params (enemy :type Enemy%20Char%20Base%20BP%20Class%20Reference))
  (Utilities|Casting|CastToenemyCharPiranha_BPClass enemy
    (:then
      (return (Variables|Default|GetpirahnaPool)))
    (:CastFailed
      (Development|PrintString "invalid pool"))))

(fn SendtoPool
  (params (enemy :type Enemy%20Char%20Base%20BP%20Object%20Reference))
  (Rendering|SetActorHiddenInGame enemy true)
  (Transformation|SetActorLocation enemy "0, 0, 0" false false)
  (bind _enemypool (CallFunction|SelectPool (Utilities|GetClass enemy)))
  (Utilities|Array|Add _enemypool enemy)
  (Development|PrintString "sent to pool"))