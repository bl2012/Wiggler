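; Player-steered worm towed on a rope behind the ChrisCraft boat, sliding sideways along a spline.
; Construction attaches it to the first boat's SpringArm; BeginPlay starts it mid-spline, looping its animation.
; MoveSide input steps spline distance and builds momentum from hold time, which Tick applies, clamps and decays while lerping CharHolder toward the spline point.
; Ending overlap with a track_BP calls that track's WormCollisionStuff with the boat.
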(event EventBeginPlay
  (bind _splinepath (Variables|Default|GetSplinePath))
  (bind _returnvalue (Spline|GetSplineLength _splinepath))
  ;[1 1 1] play bobbing anim
  (Components|Animation|PlayAnimation (Variables|Default|Getworm_char) "/Game/Characters/worm_char_Anim.worm_char_Anim" true)
  ;[1 1 1] start worm halfway along spline
  (Variables|Default|SetDist_Along_Spline (/ _returnvalue 2.0))
  ;[1 1 1] interval is 1/100 of spline
  (Variables|Default|SetSpline_Interval (/ _returnvalue 1e+02))
  (Variables|Default|Setaxis_time 0.0)
  (Class|CableComponent|SetAttachEndto (Variables|Default|Getrope) (Variables|Default|GetMyBoat) "rope_attach" "None")
  (Development|PrintString "wormy"))

(event Collision|EventActorEndOverlap
  (params (OtherActor :type Actor%20Object%20Reference))
  ;[0.9238 0.624 1 1 25] Actor End Overlap with Track: execute the worm collision stuff from the boat blueprint
  (bind _astrack_bp (Utilities|Casting|CastTotrack_BP OtherActor))
  (Default|WormCollisionStuff _astrack_bp (Variables|Default|GetMyBoat)))

(event EventTick
  (params (DeltaSeconds :type Float%20%28single-precision%29))
  (bind _splinepath (Variables|Default|GetSplinePath))
  (bind _char_holder (Variables|Default|Getchar_holder))
  (bind _returnvalue (Spline|GetSplineLength _splinepath))
  ;[0.9923 1 0.4156 1 50] Event tick: Move worm according to momentum, momentum moves toward zero
  ;;[1 1 1] if movement is valid, set it as the distance along spline
  (if (and (>= _returnvalue (+ (Variables|Default|GetDist_Along_Spline) (Variables|Default|Getmomentum))) (<= 0.0 (+ (Variables|Default|GetDist_Along_Spline) (Variables|Default|Getmomentum))))
    (Variables|Default|SetDist_Along_Spline (+ (Variables|Default|GetDist_Along_Spline) (Variables|Default|Getmomentum)))
    ;;[1 1 1] put worm at the previously established distance along the SplinePath
    (Transformation|SetWorldLocation _char_holder (Math|Vector|Lerp(Vector) (Transformation|GetWorldLocation _char_holder) (Spline|GetLocationatDistanceAlongSpline _splinepath (Variables|Default|GetDist_Along_Spline) "World") 0.1) false false :!label _label)
    ;;[1 1 1] momentum moves toward zero
    (if (and (> (Math|Float|Absolute(Float) (- (Variables|Default|Getmomentum) (* (Variables|Default|Getmomentum) 0.1))) 0.0) (> 1.0 (Math|Float|Absolute(Float) (- (Variables|Default|Getmomentum) (* (Variables|Default|Getmomentum) 0.1)))))
      (Variables|Default|Setmomentum (Math|Conversions|ToFloat(Integer) (Math|Float|Truncate (- (Variables|Default|Getmomentum) (* (Variables|Default|Getmomentum) 0.1)))))
      (else
        (Variables|Default|Setmomentum (- (Variables|Default|Getmomentum) (* (Variables|Default|Getmomentum) 0.1)))))
    (else
      (Utilities|FlowControl|Sequence
        (:then_0
          ;;[1 1 1] if movement would put distance past spline length, set dist to spline length
          (if (not (>= _returnvalue (+ (Variables|Default|GetDist_Along_Spline) (Variables|Default|Getmomentum))))
            (Variables|Default|SetDist_Along_Spline _returnvalue)
            (goto _label)))
        (:then_1
          ;;[1 1 1] if movement would put distance past zero, set distance to zero
          (if (not (<= 0.0 (+ (Variables|Default|GetDist_Along_Spline) (Variables|Default|Getmomentum))))
            (Variables|Default|SetDist_Along_Spline 0.0)
            (goto _label)))))))

(event Input|AxisEvents|InputAxisMoveSide
  (params (AxisValue :type Float%20%28single-precision%29))
  (bind _returnvalue (Utilities|Time|GetWorldDeltaSeconds))
  (bind _char_holder (Variables|Default|Getchar_holder))
  (bind _spline_interval (Variables|Default|GetSpline_Interval))
  (bind _returnvalue_2 (* _returnvalue 1e+01))
  ;[0.3781 0.9088 1 1 50] InputAxis: MoveSide
  (Math|Float|CompareFloat AxisValue 0.0
    (:>
      ;;[1 1 1] axis input is positive -> add spline interval to distance along spline
      (if (> (Spline|GetSplineLength (Variables|Default|GetSplinePath)) (Variables|Default|GetDist_Along_Spline))
        (Variables|Default|SetDist_Along_Spline (+ (Variables|Default|GetDist_Along_Spline) _spline_interval))
        ;;[1 1 1] calculate positive axis time
        (Variables|Default|Setaxis_time (+ (Variables|Default|Getaxis_time) _returnvalue_2)))
      ;;[1 1 1] add axis time to momentum
      (Variables|Default|Setmomentum (+ (Variables|Default|Getmomentum) (Variables|Default|Getaxis_time)) :!label _label))
    (:==
      ;;[0.9221 1 0.1051] check for end of spline
      (Variables|Default|Setaxis_time 0.0))
    (:<
      ;;[1 1 1] axis input is negative -> subtract spline interval from dist along spline
      (if (< 0.0 (Variables|Default|GetDist_Along_Spline))
        (Variables|Default|SetDist_Along_Spline (- (Variables|Default|GetDist_Along_Spline) _spline_interval))
        ;;[1 1 1] calculate negative axis time
        (Variables|Default|Setaxis_time (* (+ (Math|Float|Absolute(Float) (Variables|Default|Getaxis_time)) _returnvalue_2) -1.0))
        (goto _label)
        (else
          (goto _label)))))
  ;;[1 1 1] set new location along spline
  (Transformation|SetWorldLocation _char_holder (Math|Vector|Lerp(Vector) (Transformation|GetWorldLocation _char_holder) (Spline|GetLocationatDistanceAlongSpline (Variables|Default|GetSplinePath) (Variables|Default|GetDist_Along_Spline) "World") 0.1) false false))

(fn ConstructionScript
  (bind _outactors (Actor|GetAllActorsOfClass "/Game/VehicleBP/ChrisCraft/ChrisCraft_Blueprint.ChrisCraft_Blueprint_C"))
  (Transformation|AttachComponentToComponent (Variables|/Game/VehicleBP/ChrisCraft/ChrisCraft_Blueprint.ChrisCraft_Blueprint_C|GetSpringArm (Utilities|Array|Get(acopy) _outactors)) "None" "SnapToTarget" "SnapToTarget" "SnapToTarget" false)
  (Variables|Default|SetMyBoat (Utilities|Array|Get(acopy) _outactors)))