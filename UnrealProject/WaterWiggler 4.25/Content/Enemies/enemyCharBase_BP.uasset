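; Base enemy character Blueprint that senses the player's ChrisCraft pawn and is meant to be pooled through GameMode_wiggler.
; PawnSensing only prints when it sees the player, and ending overlap with a Worm_Blueprint destroys the actor outright.
; DisableEnemy returns it to the pool but is only called from disconnected nodes, including an unfinished AIMoveTo.
; AttackPlayer, not called here, sets an AttackSpline point to the mesh's relative location.
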(event OnSeePawn(PawnSensing)
  (params (Pawn :type Pawn%20Object%20Reference))
  (Utilities|Casting|CastToChrisCraft_Blueprint Pawn)
  (Development|PrintString "I see you"))

(event EventBeginPlay
  (bind _outactors (Actor|GetAllActorsOfClass "/Game/VehicleBP/ChrisCraft/ChrisCraft_Blueprint.ChrisCraft_Blueprint_C")))

(event EventTick
  (params (DeltaSeconds :type Float%20%28single-precision%29)))

(event Collision|EventActorEndOverlap
  (params (OtherActor :type Actor%20Object%20Reference))
  (Utilities|Casting|CastToWorm_Blueprint OtherActor)
  (Actor|DestroyActor))

(fn ConstructionScript)

(fn DisableEnemy
  (bind _returnvalue (Game|GetGameMode))
  (bind _asgame_mode_wiggler (Utilities|Casting|CastToGameMode_wiggler _returnvalue)
    (:then
      (Default|SendtoPool _asgame_mode_wiggler self))
    (:CastFailed
      (Development|PrintString (Utilities|String|Append "Game Mode Incorrect: " (Utilities|GetDisplayName _returnvalue))))))

(fn AttackPlayer
  (Development|PrintString "attacking")
  (Spline|SetLocationatSplinePoint (Variables|Default|Getattack_spline) 0 (Variables|/Script/Engine.SceneComponent|GetRelativeLocation (Variables|Character|GetMesh)) "Local" true))